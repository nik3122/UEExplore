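; GA_Roll is a player gameplay ability for a roll that temporarily suspends targeting.
; On activation while targeting, it clears the player's targeting flag and rotates the character to face its movement velocity.
; If that rotation succeeds, it flags retargeting and runs the parent ability's activation, which also runs directly when not targeting.
; When the ability ends, that flag restores targeting and is never reset here.
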(event `self.K2_ActivateAbility`
  (bind _returnvalue (`GameplayStatics.GetPlayerCharacter` 0))
  (bind _playercharacter (`self.PlayerCharacter`))
  (bind _asbp_player_character (cast `/Game/Blueprints/BP_PlayerCharacter` _returnvalue))
  (set `self.PlayerCharacter` _asbp_player_character)
  (if (`/Game/Blueprints/BP_CharacterBase.Is Targeting` _asbp_player_character)
    (set `/Game/Blueprints/BP_CharacterBase.Is Targeting` false _playercharacter)
    (bind _returnvalue_2 (`Actor.K2_SetActorRotation` _playercharacter (`KismetMathLibrary.Conv_VectorToRotator` (`MovementComponent.Velocity` (`Pawn.GetMovementComponent` _returnvalue))) false))
    (if _returnvalue_2
      (set `self.RetargetOnEnd` true)
      (`parent.K2_ActivateAbility` :!label _label))
    (else
      (goto _label))))

(event `self.K2_OnEndAbility`
  (params (bWasCancelled :type Boolean))
  (if (`self.RetargetOnEnd`)
    (set `/Game/Blueprints/BP_CharacterBase.Is Targeting` true (`self.PlayerCharacter`))))