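; GA_Shoot is a player Gameplay Ability that fires a BP_BallProjectile from its owner.
; On activation it commits the ability, spawns the ball just in front of the owner actor and ends, with no end call if the commit fails.
; The ball receives InitialSpeed and a 2D-normalized forward direction, so the ShootSpeed multiplier applied before normalizing does not set its speed.
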(event `self.K2_ActivateAbility`
  (bind _returnvalue_owneractor (break `GameplayAbilityActorInfo` (`self.GetActorInfo`)))
  (bind _returnvalue (`Actor.GetActorForwardVector` _returnvalue_owneractor))
  (bind _returnvalue_2 (`self.K2_CommitAbility`))
  (if _returnvalue_2
    (`|SpawnActorFromClass` "/Game/Blueprints/Weapons/BP_BallProjectile.BP_BallProjectile_C" (`KismetMathLibrary.MakeTransform` (+ (`Actor.K2_GetActorLocation` _returnvalue_owneractor) (* _returnvalue 100.0))) "Undefined" "OverrideRootScale" _returnvalue_owneractor (`self.Initial Speed`) (`KismetMathLibrary.Vector_Normal2D` (* _returnvalue (`self.ShootSpeed`))) null)
    (`self.K2_EndAbility`)))