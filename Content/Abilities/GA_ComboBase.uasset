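; Base gameplay ability for a montage-driven combo attack that chains steps from the Montages array by ComboIndex.
; Gameplay events open and close an input window; a press inside it advances the combo on window exit.
; The first step commits the full ability, later steps only cost.
; Hit events apply the mapped effect to targets; the task-cleanup loop over ActiveTaskList is never run.
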(event `OnCombo`
  (bind _returnvalue (`self.K2_CommitAbilityCost` false))
  (if _returnvalue
    (bind _montage (`self.GetMontageToPlay` :!label _label))
    (`AbilityTask_PlayMontageAndWait.CreatePlayMontageAndWaitProxy` "None" _montage
      (:`then`
        (bind (_asynctaskproxy _payload) (`AbilityTask_WaitGameplayEvent.WaitGameplayEvent` (struct :`TagName` "Ability.Hit") null)
          (:`then`
            (`KismetArrayLibrary.Array_Add` (`self.ActiveTaskList`) _asynctaskproxy)
            (set `self.In Combo Window` false)
            (bind _asynctaskproxy_2 (`AbilityTask_WaitGameplayEvent.WaitGameplayEvent` (struct :`TagName` "Ability.Combo.Enter") null)
              (:`then`
                (`KismetArrayLibrary.Array_Add` (`self.ActiveTaskList`) _asynctaskproxy_2)
                (bind _asynctaskproxy_3 (`AbilityTask_WaitGameplayEvent.WaitGameplayEvent` (struct :`TagName` "Ability.Combo.Exit") null)
                  (:`then`
                    (`KismetArrayLibrary.Array_Add` (`self.ActiveTaskList`) _asynctaskproxy_3))
                  (:`EventReceived`
                    (set `self.In Combo Window` false)
                    (if (`self.Combo Granted`)
                      (set `self.Combo Granted` false)
                      (`/Engine/EditorBlueprintResources/StandardMacros.IncrementInt` (`self.Combo Index`)
                        (:`  `
                          (`self.OnCombo`)))))))
              (:`EventReceived`
                (set `self.Combo Granted` false)
                (set `self.In Combo Window` true)
                (bind _asynctaskproxy_4 (`AbilityTask_WaitInputPress.WaitInputPress` false)
                  (:`then`
                    (`KismetArrayLibrary.Array_Add` (`self.ActiveTaskList`) _asynctaskproxy_4))
                  (:`OnPress`
                    (if (`self.In Combo Window`)
                      (set `self.Combo Granted` true)))))))
          (:`EventReceived`
            (bind (_eventtag _instigator _target _optionalobject _optionalobject2 _contexthandle _instigatortags _targettags _eventmagnitude _targetdata) (break `GameplayEventData` _payload))
            (`self.BP_ApplyGameplayEffectToTarget` _targetdata (`BlueprintMapLibrary.Map_Find` (`self.GameplayEffectMap`) _eventtag)))))
      (:`OnCompleted`
        (`self.K2_EndAbility` :!label _label_2))
      (:`OnBlendOut`
        (if (not (`self.Combo Granted`)) :!label _label_3
          (goto _label_2)))
      (:`OnInterrupted`
        (goto _label_3))
      (:`OnCancelled`
        (goto _label_3)))))

(event `self.K2_ActivateAbility`
  (`self.ResetComboState`)
  (bind _returnvalue (`self.K2_CommitAbility`))
  (if _returnvalue
    (goto _label)))

(event `self.K2_OnEndAbility`
  (params (bWasCancelled :type Boolean))
  (`self.ResetComboState`))

(fn `GetMontageToPlay`
  (returns (Montage :type "AnimMontage Object Reference"))
  (return (`|GetArrayItem` (`self.Montages`) (`self.Combo Index`))))

(fn `ResetComboState`
  (set `self.Combo Index` 0)
  (set `self.Combo Granted` false))