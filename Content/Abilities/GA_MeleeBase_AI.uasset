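; Base melee Gameplay Ability for AI that plays a combo of attack montages.
; Each step commits the ability, plays the montage at the combo index, then waits for an Ability.Combo.ExecuteAI gameplay event to chain the next.
; A montage completing or blending out leads to an optional cooldown montage or delay before ending; interruption ends it directly.
; On end, it resets the index and stops all tracked async tasks.
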(event `Combo`
  (bind _asynctasks (`self.AsyncTasks`))
  (bind _cooldown_montage (`self.Cooldown Montage`))
  (set `self.InCombo` true)
  (bind _returnvalue (`self.K2_CommitAbility` :!label _label))
  (if _returnvalue
    (bind _montage (`self.GetMontageToPlay`))
    (bind _asynctaskproxy (`AbilityTask_PlayMontageAndWait.CreatePlayMontageAndWaitProxy` "None" _montage)
      (:`then`
        (`KismetArrayLibrary.Array_Add` (`self.AsyncTasks`) _asynctaskproxy)
        (`/Engine/EditorBlueprintResources/StandardMacros.IncrementInt` (`self.Combo Index`)
          (:`  `
            (bind _asynctaskproxy_2 (`AbilityTask_WaitGameplayEvent.WaitGameplayEvent` (struct :`TagName` "Ability.Combo.ExecuteAI") null)
              (:`then`
                (`KismetArrayLibrary.Array_Add` (`self.AsyncTasks`) _asynctaskproxy_2))
              (:`EventReceived`
                (`self.Combo`))))))
      (:`OnCompleted`
        (if (`KismetSystemLibrary.IsValid` _cooldown_montage) :!label _label_2
          (bind _asynctaskproxy_3 (`AbilityTask_PlayMontageAndWait.CreatePlayMontageAndWaitProxy` "None" _cooldown_montage)
            (:`then`
              (`KismetArrayLibrary.Array_Add` _asynctasks _asynctaskproxy_3))
            (:`OnCompleted`
              (`self.K2_EndAbility` :!label _label_3))
            (:`OnInterrupted`
              (goto _label_3))
            (:`OnCancelled`
              (goto _label_3)))
          (elif (> (`self.Cooldown Delay`) 0.0)
            (bind _asynctaskproxy_4 (`AbilityTask_WaitDelay.WaitDelay` (`self.Cooldown Delay`))
              (:`then`
                (`KismetArrayLibrary.Array_Add` _asynctasks _asynctaskproxy_4))
              (:`OnFinish`
                (goto _label_3)))
            (else
              (goto _label_3)))))
      (:`OnBlendOut`
        (goto _label_2))
      (:`OnInterrupted`
        (`self.K2_EndAbility` :!label _label_4))
      (:`OnCancelled`
        (goto _label_4)))
    (else
      (`self.K2_EndAbility`))))

(event `self.K2_ActivateAbility`
  (set `self.InCombo` false)
  (goto _label))

(event `self.K2_OnEndAbility`
  (params (bWasCancelled :type Boolean))
  (set `self.Combo Index` 0)
  (for _array_element (`self.AsyncTasks`)
    (`/Engine/EditorBlueprintResources/StandardMacros.IsValid` _array_element
      (:`Is Valid`
        (`GameplayTask.EndTask` _array_element))))
  (`self.AbilityEnded`))

(fn `GetMontageToPlay`
  (returns (Montage :type "AnimMontage Object Reference"))
  (bind _combo_index (`self.Combo Index`))
  (`KismetSystemLibrary.PrintString` (`KismetStringLibrary.Conv_IntToString` _combo_index))
  (return (`|GetArrayItem` (`self.Montages`) _combo_index)))