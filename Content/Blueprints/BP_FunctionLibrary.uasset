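; Blueprint function library with shared helpers for attack ranges and menu handling.
; The range helpers pick a random attack range enum value from the entry count and map close, mid and long values to fixed distances.
; EnterMenu adds a widget to the viewport, optionally pauses, and gives player 0 a cursor with game-and-UI input focused on it.
; ExitMenu removes the widget, hides the cursor, always unpauses and restores game-only input.
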(fn `EnterMenu`
  (params (Widget :type "UserWidget Object Reference") (PauseGame :type Boolean))
  (bind _returnvalue (`GameplayStatics.GetPlayerController` (`local.__WorldContext`)))
  (`GameplayStatics.SetGamePaused` (`local.__WorldContext`) PauseGame)
  (set `PlayerController.bShowMouseCursor` true _returnvalue)
  (`WidgetBlueprintLibrary.SetInputMode_GameAndUIEx` _returnvalue (`local.Widget`))
  (`UserWidget.AddToViewport` (`local.Widget`) 0))

(fn `ExitMenu`
  (params (Widget :type "UserWidget Object Reference"))
  (bind ___worldcontext (`local.__WorldContext`))
  (bind _returnvalue (`GameplayStatics.GetPlayerController` ___worldcontext))
  (`Widget.RemoveFromParent` Widget)
  (set `PlayerController.bShowMouseCursor` false _returnvalue)
  (`GameplayStatics.SetGamePaused` ___worldcontext)
  (`WidgetBlueprintLibrary.SetInputMode_GameOnly` _returnvalue))

(fn `Get Random Attack Range`
  (returns (RandomAttackRange :type "/Game/Blueprints/Combat/EAttackRange Enum"))
  (return (cast `/Game/Blueprints/Combat/EAttackRange` (`KismetMathLibrary.Conv_IntToByte` (`KismetMathLibrary.RandomIntegerInRange` 0 (- (enumcount `/Game/Blueprints/Combat/EAttackRange`) 1))))))

(fn `GetAttackRangeFromEnum`
  (params (AttackRangeEnum :type "/Game/Blueprints/Combat/EAttackRange Enum" :default "NewEnumerator0"))
  (returns (AttackRange :type "Float (double-precision)"))
  (locals (LAttackRange :type "Float (double-precision)"))
  (switch `/Game/Blueprints/Combat/EAttackRange` AttackRangeEnum
    (:`NewEnumerator0`
      (set `local.LAttackRange` 100.0))
    (:`NewEnumerator1`
      (set `local.LAttackRange` 500.0))
    (:`NewEnumerator2`
      (set `local.LAttackRange` 1000.0)))
  (return (`local.LAttackRange`)))