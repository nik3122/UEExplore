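; Enemy AI controller that runs BT_Enemy on possession and tracks the player through AI perception.
; Sensing a Player-tagged actor sets the line-of-sight and enemy blackboard keys; other updates start a timer that clears both, giving a grace period after losing sight.
; Jump events launch the possessed EnemyA_BP with a scaled velocity, draw a debug arrow and toggle IsJumping.
; PlayAttack is an empty stub.
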(event `self.ReceivePossess`
  (params (PossessedPawn :type "Pawn Object Reference"))
  (set `self.Possessed Pawn` PossessedPawn)
  (`self.RunBehaviorTree` "/Game/AI/BT_Enemy.BT_Enemy"))

(event `self.AIPerception.OnTargetPerceptionUpdated`
  (params (Actor :type "Actor Object Reference") (Stimulus :type "AIStimulus Structure"))
  (bind _blackboard (`self.Blackboard`))
  (set `self.SensedActor` Actor)
  (if (and (`self.ActorHasTag` (`self.SensedActor`) "Player") (`.bSuccessfullySensed` (break `AIStimulus` Stimulus)))
    (`KismetSystemLibrary.K2_ClearAndInvalidateTimerHandle` (`self.EnemyTimer`))
    (`BlackboardComponent.SetValueAsBool` _blackboard (`self.HasLineOfSight`) true)
    (`BlackboardComponent.SetValueAsObject` _blackboard (`self.EnemyActor`) (`self.SensedActor`))
    (else
      (bind _returnvalue (`KismetSystemLibrary.K2_SetTimerDelegate` (delegate `StartEnemyTimer`) (`self.LineOfSightTimer`)))
      (set `self.EnemyTimer` _returnvalue))))

(event `StartEnemyTimer`
  (bind _blackboard (`self.Blackboard`))
  (`BlackboardComponent.SetValueAsBool` _blackboard (`self.HasLineOfSight`) false)
  (`BlackboardComponent.SetValueAsObject` _blackboard (`self.EnemyActor`) null))

(event `OnJump`
  (params (LaunchVelocity :type "Vector Structure"))
  (bind _returnvalue (* LaunchVelocity 10.0))
  (bind _possessed_pawn (`self.Possessed Pawn`))
  (bind _returnvalue_2 (`self.K2_GetActorLocation` _possessed_pawn))
  (bind _asenemy_a_bp (cast `/Game/Blueprints/EnemyA_BP` _possessed_pawn))
  (`Character.LaunchCharacter` _asenemy_a_bp _returnvalue false false)
  (set `self.IsJumping` true)
  (`KismetSystemLibrary.DrawDebugArrow` _returnvalue_2 (- _returnvalue _returnvalue_2) 100.0 (struct :`R` 0.600083 :`G` 0.053068 :`B` 0.122905 :`A` 1.0) 5.0 5.0))

(event `OnJUmpEnd`
  (bind _asenemy_a_bp (cast `/Game/Blueprints/EnemyA_BP` (`self.Possessed Pawn`)))
  (`Character.StopJumping` _asenemy_a_bp)
  (set `self.IsJumping` false))

(fn `Play Attack`
  (params (AttackType :type "/Game/Blueprints/EAttackRange Enum" :default "NewEnumerator1") (NewParam :type "/Game/Blueprints/EAttackRange Enum" :default "NewEnumerator0")))

(fn `UserConstructionScript`)