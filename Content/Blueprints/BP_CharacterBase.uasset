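; Base character Blueprint providing shared combat behavior: ability hit reactions, poise break, lock-on and an alive-and-unpaused check for ability use.
; Taking a hit sends an Ability.Hit gameplay event to the instigator and drives a material hit flash, while poise break plays a DoOnce-gated montage.
; Tick yaws toward the lock-on target until it exceeds range; target search is a stub returning false.
; A helper repositions the character around a target actor.
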(event `self.OnPoiseBreak`
  (`/Engine/EditorBlueprintResources/StandardMacros.DoOnce` false :!label _label
    (:`Completed`
      (`|PlayMontage` (`self.Mesh`) (`self.PoiseBreakMontage`)
        (:`OnCompleted`
          (goto _label :!via `Reset`))
        (:`OnInterrupted`
          (goto _label :!via `Reset`))))))

(event `/Game/Blueprints/IBP_IDamageable.TakeHitFromAbility`
  (params (Instigator :type "Actor Object Reference"))
  (bind _mesh (`self.Mesh`))
  ;[1 1 1] IDamageable Implementation
  (`AbilitySystemBlueprintLibrary.SendGameplayEventToActor` Instigator (struct :`TagName` "Ability.Hit") (make `GameplayEventData` (struct) Instigator null null null (struct) (struct) (struct) 0.0 (`AbilitySystemBlueprintLibrary.AbilityTargetDataFromActor` self)))
  (`MeshComponent.SetScalarParameterValueOnMaterials` _mesh "HitFlashFrequency" 0.5)
  (`MeshComponent.SetScalarParameterValueOnMaterials` _mesh "TimeOfHit" (`GameplayStatics.GetTimeSeconds`)))

(event `self.ReceiveTick`
  (params (DeltaSeconds :type "Float (single-precision)"))
  ;[1 1 1] LockOn
  (if (`self.Is Targeting`)
    (if (> (`KismetMathLibrary.Vector_Distance` (`self.K2_GetActorLocation`) (`self.K2_GetActorLocation` (`self.LockOnTarget`))) (`self.MaxTargetingDistance`))
      (set `self.Is Targeting` false)
      (else
        (`self.LookAtTarget` (`self.LockOnTarget`))))))

(fn `CanUseAbility`
  (returns (Result :type Boolean))
  ;[1 1 1] Don't allow while dead or paused. Subclasses can change this
  (return (and (`self.IsAlive`) (not (`GameplayStatics.IsGamePaused`)))))

(fn `IsAlive`
  (returns (Return :type Boolean))
  (return (> (`self.GetHealth`) 0.0)))

(fn `LookAtTarget`
  (params (TargetActor :type "Actor Object Reference"))
  (bind (_returnvalue_roll _returnvalue_pitch) (`KismetMathLibrary.BreakRotator` (`self.K2_GetActorRotation`)))
  (bind (_returnvalue_roll_2 _returnvalue_pitch_2 _returnvalue_yaw) (`KismetMathLibrary.BreakRotator` (`KismetMathLibrary.FindLookAtRotation` (`self.K2_GetActorLocation`) (`self.K2_GetActorLocation` TargetActor))))
  (`/Engine/EditorBlueprintResources/StandardMacros.IsValid` TargetActor
    (:`Is Valid`
      (`self.K2_SetActorRotation` (`KismetMathLibrary.MakeRotator` _returnvalue_roll _returnvalue_pitch _returnvalue_yaw)))))

(fn `RotateAroundPoint`
  (params (Radius :type "Float (double-precision)") (Rate :type "Float (double-precision)") (Angle :type "Float (double-precision)") (TargetLocation :type "Vector Structure") (TargetActor :type "Actor Object Reference"))
  (returns (Success :type Boolean))
  (locals (LLocation :type "Vector Structure") (LRadius :type "Float (double-precision)") (LRate :type "Float (double-precision)") (LAngle :type "Float (double-precision)") (LTargetActor :type "Actor Object Reference"))
  (set `local.LLocation` TargetLocation)
  (set `local.LRadius` Radius)
  (set `local.LRate` Rate)
  (set `local.LAngle` Angle)
  (bind _output_get (set `local.LTargetActor` TargetActor))
  (`/Engine/EditorBlueprintResources/StandardMacros.IsValid` _output_get
    (:`Is Valid`
      (set `local.LLocation` (`self.K2_GetActorLocation` _output_get))
      (bind (_sweephitresult _returnvalue) (`self.K2_SetActorLocation` (+ (`local.LLocation`) (`KismetMathLibrary.RotateAngleAxis` (`KismetMathLibrary.MakeVector` (`local.LRadius`)) (+ (`local.LAngle`) (`local.LRate`)) (0.0 0.0 1.0)))))
      (return _returnvalue))))

(fn `TryFindLockOnTarget`
  (returns (FoundTargetActor :type "Actor Object Reference") (Found :type Boolean))
  (return null false))

(fn `UserConstructionScript`)