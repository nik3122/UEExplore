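; BP_Character is a base character Blueprint that provides shared ability checks and an orbit-positioning helper.
; CanUseAbility, which subclasses can change, requires health above zero via IsAlive and an unpaused game.
; DoMeleeAttack runs that check but performs no attack here, and the event graph is empty.
; RotateAroundPoint places the character at a radius around a valid target actor, rotating the offset about Z by angle plus rate.
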(event `self.ReceiveTick`
  (params (DeltaSeconds :type "Float (single-precision)")))

(fn `CanUseAbility`
  (returns (Result :type Boolean))
  ;[1 1 1] Don't allow while dead or paused. Subclasses can change this
  (bind _return (`self.IsAlive`))
  (return (and _return (not (`GameplayStatics.IsGamePaused`)))))

(fn `DoMeleeAttack`
  (bind _result (`self.CanUseAbility`))
  (if _result
    _))

(fn `IsAlive`
  (returns (Return :type Boolean))
  (bind _returnvalue (`self.GetHealth`))
  (return (> _returnvalue 0.0)))

(fn `RotateAroundPoint`
  (params (Radius :type "Float (double-precision)") (Rate :type "Float (double-precision)") (Angle :type "Float (double-precision)") (TargetLocation :type "Vector Structure") (TargetActor :type "Actor Object Reference"))
  (returns (Success :type Boolean))
  (locals (LLocation :type "Vector Structure") (LRadius :type "Float (double-precision)") (LRate :type "Float (double-precision)") (LAngle :type "Float (double-precision)") (LTargetActor :type "Actor Object Reference"))
  (set `local.LLocation` TargetLocation)
  (set `local.LRadius` Radius)
  (set `local.LRate` Rate)
  (set `local.LAngle` Angle)
  (bind _output_get (set `local.LTargetActor` TargetActor))
  (`/Engine/EditorBlueprintResources/StandardMacros.IsValid` _output_get
    (:`Is Valid`
      (set `local.LLocation` (`self.K2_GetActorLocation` _output_get))
      (bind (_sweephitresult _returnvalue) (`self.K2_SetActorLocation` (+ (`local.LLocation`) (`KismetMathLibrary.RotateAngleAxis` (`KismetMathLibrary.MakeVector` (`local.LRadius`)) (+ (`local.LAngle`) (`local.LRate`)) (0.0 0.0 1.0)))))
      (return _returnvalue))))

(fn `UserConstructionScript`)