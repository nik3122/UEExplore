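; AI controller for enemies that runs a behavior tree on possession and feeds it perception results through the Blackboard.
; Successfully sensing a Player-tagged actor cancels the timer and sets TargetActor and HasLineOfSight.
; Any other perception update starts a grace timer that clears both keys when it expires.
; A ComboWindowToggle event mirrors the combo window state into the Blackboard.
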(event `self.ReceivePossess`
  (params (PossessedPawn :type "Pawn Object Reference"))
  (set `self.Possessed Pawn` PossessedPawn)
  (`self.RunBehaviorTree` (`self.BehaviorTree`)))

(event `self.AIPerception.OnTargetPerceptionUpdated`
  (params (Actor :type "Actor Object Reference") (Stimulus :type "AIStimulus Structure"))
  (bind _blackboard (`self.Blackboard`))
  (`/Engine/EditorBlueprintResources/StandardMacros.IsValid` (`self.BehaviorTree`)
    (:`Is Valid`
      (if true
        (set `self.SensedActor` Actor)
        (if (and (`self.ActorHasTag` (`self.SensedActor`) "Player") (`.bSuccessfullySensed` (break `AIStimulus` Stimulus)))
          (`KismetSystemLibrary.K2_ClearAndInvalidateTimerHandle` (`self.EnemyTimer`))
          (`BlackboardComponent.SetValueAsBool` _blackboard (`self.HasLineOfSight`) true)
          (`BlackboardComponent.SetValueAsObject` _blackboard (`self.TargetActor`) (`self.SensedActor`))
          (else
            (bind _returnvalue (`KismetSystemLibrary.K2_SetTimerDelegate` (delegate `StartEnemyTimer`) (`self.LineOfSightTimer`)))
            (set `self.EnemyTimer` _returnvalue)))))))

(event `StartEnemyTimer`
  (bind _blackboard (`self.Blackboard`))
  (`BlackboardComponent.SetValueAsBool` _blackboard (`self.HasLineOfSight`) false)
  (`BlackboardComponent.SetValueAsObject` _blackboard (`self.TargetActor`) null))

(event `ComboWindowToggle`
  (params (Active :type Boolean))
  (`BlackboardComponent.SetValueAsBool` (`self.Blackboard`) (`self.InComboWindow`) Active))

(fn `GetControlledCharacter`
  (params (ControlledPawn :type "Pawn Object Reference"))
  (returns (ControlledCharacter :type "Character Object Reference"))
  (bind _ascharacter (cast `Character` ControlledPawn))
  (return _ascharacter))

(fn `UserConstructionScript`)