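; Base melee weapon actor that deals hits to damageable actors during an attack window.
; Attack window events toggle the attacking flag and the collider's query-only collision.
; Overlaps skip actors of the instigator's class and send a take-hit interface message with the instigator, plus a debug "HIT" print.
; A DoOnce gate limits repeat hits, resetting shortly after any overlap ends.
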(event `OnEnterAttackWindow`
  (set `self.IsAttacking` true)
  (`PrimitiveComponent.SetCollisionEnabled` (`self.Collider`) "QueryOnly"))

(event `OnExitAttackWindow`
  (set `self.IsAttacking` false)
  (`PrimitiveComponent.SetCollisionEnabled` (`self.Collider`) "NoCollision"))

(event `self.ReceiveActorBeginOverlap`
  (params (OtherActor :type "Actor Object Reference"))
  (bind _returnvalue (`self.GetInstigator`))
  ;[1 1 1] Don't collide with self
  (if (and (!= (`GameplayStatics.GetObjectClass` OtherActor) (`GameplayStatics.GetObjectClass` _returnvalue)) (`KismetSystemLibrary.DoesImplementInterface` OtherActor "/Game/Blueprints/IBP_IDamageable.IBP_IDamageable_C") (`self.IsAttacking`))
    (`/Engine/EditorBlueprintResources/StandardMacros.DoOnce` false :!label _label
      (:`Completed`
        (message `/Game/Blueprints/IBP_IDamageable.TakeHitFromAbility` OtherActor _returnvalue)
        (`KismetSystemLibrary.PrintString` "HIT" true true (struct :`R` 0.148991 :`G` 1.0 :`B` 0.224322 :`A` 1.0))))))

(event `self.ReceiveActorEndOverlap`
  (params (OtherActor :type "Actor Object Reference"))
  (`KismetSystemLibrary.Delay` 0.2)
  (goto _label :!via `Reset`))

(fn `UserConstructionScript`)