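; BP_BallProjectile is a ball projectile Blueprint that triggers interactable actors it overlaps.
; On overlap, it calls the parent handler, then checks whether the other actor implements IBP_Interactable.
; If so, it sends InteractMessage with player 0's BP_PlayerCharacter as the argument, provided that cast succeeds, regardless of who fired the ball.
; BeginPlay, Tick and the construction script add no logic of their own.
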(event `self.ReceiveActorBeginOverlap`
  (params (OtherActor :type "Actor Object Reference"))
  (`parent.ReceiveActorBeginOverlap` OtherActor)
  (if (`KismetSystemLibrary.DoesImplementInterface` OtherActor "/Game/Blueprints/IBP_Interactable.IBP_Interactable_C")
    (bind _asbp_player_character (cast `/Game/Blueprints/BP_PlayerCharacter` (`GameplayStatics.GetPlayerCharacter` 0)))
    (message `/Game/Blueprints/IBP_Interactable.Interact` OtherActor _asbp_player_character)))

(fn `UserConstructionScript`
  (`parent.UserConstructionScript`))