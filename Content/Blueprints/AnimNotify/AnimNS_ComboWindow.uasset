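; AnimNS_ComboWindow is an animation notify state that marks a combo window for enemy AI during an animation.
; It finds the controller through the mesh owner's Instigator and casts it to BP_EnemyController.
; It calls ComboWindowToggle with true when the notify begins and false when it ends, doing nothing if the cast fails.
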(fn `Received_NotifyBegin`
  (params (MeshComp :type "SkeletalMeshComponent Object Reference") (Animation :type "AnimSequenceBase Object Reference") (TotalDuration :type "Float (double-precision)"))
  (returns (ReturnValue :type Boolean))
  (bind _asbp_enemy_controller (cast `/Game/Blueprints/BP_EnemyController` (`Pawn.GetController` (`Actor.Instigator` (`ActorComponent.GetOwner` MeshComp)))))
  (`/Game/Blueprints/BP_EnemyController.ComboWindowToggle` _asbp_enemy_controller true)
  (return false))

(fn `Received_NotifyEnd`
  (params (MeshComp :type "SkeletalMeshComponent Object Reference") (Animation :type "AnimSequenceBase Object Reference"))
  (returns (ReturnValue :type Boolean))
  (bind _asbp_enemy_controller (cast `/Game/Blueprints/BP_EnemyController` (`Pawn.GetController` (`Actor.Instigator` (`ActorComponent.GetOwner` MeshComp)))))
  (`/Game/Blueprints/BP_EnemyController.ComboWindowToggle` _asbp_enemy_controller false)
  (return false))