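; Player controller that toggles lock-on to another character when the LockOn input is pressed.
; A press asks the possessed character to find a target, stores it if it is a BP_Character, and switches that character's lock-on mode; pressing again clears it.
; A helper can yaw the control rotation toward the target, preserving pitch and roll, but its call is disconnected, so this controller never applies it.
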(event `self.ReceiveTick`
  (params (DeltaSeconds :type "Float (single-precision)")))

(event `self.ReceivePossess`
  (params (PossessedPawn :type "Pawn Object Reference")))

(event `InputAction|LockOn`
  (params (Key :type "Key Structure"))
  (bind _possessedxcharacter (`self.PossessedXCharacter`))
  (:`Pressed`
    (if (`self.LockOn`)
      (set `self.LockOnTarget` null)
      (bind _output_get (set `self.LockOn` false))
      (`/Game/Blueprints/BP_Player.SetLockOnMode` (`self.PossessedXCharacter`) _output_get)
      (else
        (bind (_foundtargetactor _found) (`/Game/Blueprints/BP_Player.TryFindLockOnTarget` _possessedxcharacter))
        (if _found
          (bind _asbp_character (cast `/Game/Blueprints/BP_Character` _foundtargetactor))
          (set `self.LockOnTarget` _asbp_character)
          (bind _output_get_2 (set `self.LockOn` true))
          (`/Game/Blueprints/BP_Player.SetLockOnMode` _possessedxcharacter _output_get_2))))))

(fn `LockRotationOnTarget`
  (params (LockOnTarget :type "Actor Object Reference"))
  (bind (_returnvalue_roll _returnvalue_pitch) (`KismetMathLibrary.BreakRotator` (`self.GetControlRotation`)))
  (bind (_returnvalue_roll_2 _returnvalue_pitch_2 _returnvalue_yaw) (`KismetMathLibrary.BreakRotator` (`KismetMathLibrary.FindLookAtRotation` (`self.K2_GetActorLocation` (`self.PossessedXCharacter`)) (`self.K2_GetActorLocation` LockOnTarget))))
  (`self.SetControlRotation` (`KismetMathLibrary.MakeRotator` _returnvalue_roll _returnvalue_pitch _returnvalue_yaw)))

(fn `UserConstructionScript`)