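; Elevator actor that travels back and forth by an offset when another actor overlaps it.
; A FlipFlop alternates the destination between current location plus and minus TargetLocation on each overlap.
; MoveComponentTo moves the root there over Duration, behind a DoOnce that resets after the move.
; The FlipFlop sits ahead of the DoOnce, so overlaps during travel still toggle the direction.
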(event `self.ReceiveActorBeginOverlap`
  (params (OtherActor :type "Actor Object Reference"))
  (bind _returnvalue (`self.K2_GetActorLocation`))
  (bind _targetlocation (`self.TargetLocation`))
  (`/Engine/EditorBlueprintResources/StandardMacros.FlipFlop`
    (:`A`
      (set `self.RelativeTargetDest` (+ _returnvalue _targetlocation)))
    (:`B`
      (set `self.RelativeTargetDest` (+ _returnvalue (* _targetlocation -1)))))
  (`/Engine/EditorBlueprintResources/StandardMacros.DoOnce` false :!label _label
    (:`Completed`
      (`KismetSystemLibrary.MoveComponentTo` (`self.DefaultSceneRoot`) (`self.RelativeTargetDest`) (struct) false false (`self.Duration`))
      (goto _label :!via `Reset`))))

(fn `UserConstructionScript`)