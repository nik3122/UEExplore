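; Jump pad actor that changes the player character's jump height while they overlap it.
; When a BP_PlayerCharacter begins overlapping, it caches the character and its original jump Z velocity, then applies the pad's own value.
; Any end overlap restores the cached velocity and clears the reference, without checking which actor left.
; The pad applies no launch itself; it only modifies the jump velocity.
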(event `self.ReceiveActorBeginOverlap`
  (params (OtherActor :type "Actor Object Reference"))
  (bind _asbp_player_character (cast `/Game/Blueprints/BP_PlayerCharacter` OtherActor))
  (bind _output_get (set `self.PlayerCharacter` _asbp_player_character))
  (bind _zvelocity (`/Game/Blueprints/BP_PlayerCharacter.GetJumpZVelocity` _output_get))
  (set `self.InitialJumpZVelocity` _zvelocity)
  (`/Game/Blueprints/BP_PlayerCharacter.SetJumpZVelocity` (`self.PlayerCharacter`) (`self.JumpZVelocity`)))

(event `self.ReceiveActorEndOverlap`
  (params (OtherActor :type "Actor Object Reference"))
  (`/Game/Blueprints/BP_PlayerCharacter.SetJumpZVelocity` (`self.PlayerCharacter`) (`self.InitialJumpZVelocity`))
  (set `self.PlayerCharacter` null))

(fn `UserConstructionScript`)