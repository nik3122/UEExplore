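; MovingActivatable_BP is an activatable mechanic that moves and rotates a mesh between its starting pose and an offset.
; Each Activate alternates through a FlipFlop between playing a timeline forward and reversing it from the end, with play rate derived from Duration.
; The timeline's ratio scales Displacement and Rotation into MovingMesh's relative transform, and its completion calls CallOnFinishActivate.
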(event `/Game/Blueprints/IBP_Activatable.Activate`
  (`TimelineComponent.SetPlayRate` (`self.MoveRatioTimeline`) (/ 1.0 (`self.Duration`)))
  (`/Engine/EditorBlueprintResources/StandardMacros.FlipFlop`
    (:`A`
      (bind (_direction _ratio) (`Timeline|MoveRatioTimeline` :!label _label)
        (:`Update`
          (`SceneComponent.K2_SetRelativeLocationAndRotation` (`self.MovingMesh`) (* (`self.Displacement`) _ratio) (* (`self.Rotation`) _ratio) false false))
        (:`Finished`
          (`self.OnFinishActivate`))))
    (:`B`
      (goto _label :!via `ReverseFromEnd`))))

(fn `UserConstructionScript`
  (`parent.UserConstructionScript`))